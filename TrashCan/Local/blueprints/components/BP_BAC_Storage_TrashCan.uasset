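; Interactable storage component for a trash can placeable that opens the owner's inventory through the CraftingGUI module.
; Activation toggles each player in an interacting list; losing selection also removes them.
; The first user in and last one out drive a multicast open state, and closing saves the owner.
; BeginPlay reloads inventory data using the owner's building persistence component IDs.
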(event Custom|CheckState
  (params (Instigator :type Player%20Controller%20Object%20Reference))
  (bind _playersinteractingwithchest (Variables|Default|GetPlayersInteractingWithChest))
  (if (Utilities|Array|ContainsItem (Variables|Default|GetPlayersInteractingWithChest) Instigator)
    (Utilities|Array|RemoveItem (Variables|Default|GetPlayersInteractingWithChest) Instigator)
    (CallFunction|CloseGui Instigator)
    (if (== (Utilities|Array|Length (Variables|Default|GetPlayersInteractingWithChest)) 0)
      (CallFunction|CloseChest))
    (else
      (if (== (Utilities|Array|Length (Variables|Default|GetPlayersInteractingWithChest)) 0)
        (Utilities|Array|Add _playersinteractingwithchest Instigator)
        (CallFunction|OpenChest)
        (else
          (Utilities|Array|Add _playersinteractingwithchest Instigator)))
      (CallFunction|OpenGui Instigator))))

(event Custom|OpenChest
  (CallFunction|MulticastOpenChest))

(event Custom|CloseChest
  (CallFunction|MulticastCloseChest)
  (Class|WorldPersistenceComponent|SaveActor (Components|GetOwner)))

(event Custom|Multicast_OpenChest
  (Variables|Default|SetOpenState true))

(event Custom|Multicast_CloseChest
  (Variables|Default|SetOpenState false))

(event Custom|CloseGui
  (params (Instigator :type Player%20Controller%20Object%20Reference))
  ;[1 1 1] Handle GUI
  (Class|ConanCharacter|SetInteractingActor (.AsConan%20Character (Utilities|Casting|CastToConanCharacter (Pawn|GetControlledPawn Instigator))) 0 "None"))

(event Custom|OpenGui
  (params (Instigator :type Player%20Controller%20Object%20Reference))
  ;[1 1 1] Handle GUI
  (Class|ConanCharacter|SetInteractingActor (.AsConan%20Character (Utilities|Casting|CastToConanCharacter (Pawn|GetControlledPawn Instigator))) (Components|GetOwner) "CraftingGUI"))

(event Custom|CheckStateAndClose
  (params (Instigator :type Player%20Controller%20Object%20Reference))
  (if (Utilities|Array|ContainsItem (Variables|Default|GetPlayersInteractingWithChest) Instigator)
    (Utilities|Array|RemoveItem (Variables|Default|GetPlayersInteractingWithChest) Instigator)
    (if (== (Utilities|Array|Length (Variables|Default|GetPlayersInteractingWithChest)) 0)
      (CallFunction|CloseChest))))

(event EventBeginPlay
  (bind _returnvalue (Components|GetOwner))
  ;[1 1 1] Begin play
  (for _array_element (Actor|GetComponentsByClass _returnvalue "/Script/ConanSandbox.ConanBuildingPersistenceComponent")
    (bind _result (|LoadInventory (Class|PersistenceComponent|GetUniqueID _array_element))
      (:OnSuccess
        (Class|LoadInventoryCallProxy|ProcessInventoryData _returnvalue _result)))))

(event EventInteractableActivate
  (params (Component :type Primitive%20Component%20Object%20Reference) (Instigator :type Player%20Controller%20Object%20Reference) (HitIndex :type Integer) (TriggeredFromRadialWheel :type Boolean))
  (CallFunction|CheckState Instigator))

(event EventInteractableSelectionChanged
  (params (IsSelected :type Boolean) (Instigator :type Player%20Controller%20Object%20Reference) (InstanceIndex :type Integer))
  (if (not IsSelected)
    (CallFunction|CheckStateandCLose Instigator)))