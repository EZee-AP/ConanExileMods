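; Placeable trash can chest Blueprint that adds an option to empty its contents.
; It extends the parent interactable radial menu with an "Empty" entry using a trash can icon.
; Clicking it finds the MDC_Component on the local player character and calls its ServerEmptyTrash with the chest's placeable inventory, routing the emptying through the player's component.
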(event Custom|EmptyTrash
  (params (menuEntry :type Radial%20Menu%20Entry%20Object%20Reference))
  (Default|ServerEmptyTrash (Utilities|Array|Get(acopy) (Actor|GetComponentsByClass (Game|GetPlayerCharacter 0) "/Game/Mods/TrashCan/MDC_Component.MDC_Component_C")) (Variables|Default|GetPlaceableInventory)))

(event EventInteractableMenu
  (params (RadialMenu :type Radial%20Menu%20Object%20Reference) (HitIndex :type Integer))
  (|CallParentFunction RadialMenu HitIndex)
  (bind _returnvalue (Class|RadialMenu|AddItem RadialMenu "Empty" "" "/Game/Mods/TrashCan/textures/T_MainRadialMenuIconTrashCan.T_MainRadialMenuIconTrashCan" "None" -1))
  (EventDispatchers|BindEventtoSignalClicked _returnvalue (delegate Custom|EmptyTrash)))

(fn ConstructionScript
  (|CallParentFunction))