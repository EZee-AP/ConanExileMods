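; Base spell actor for the magic system, providing shared setup and stacking helpers.
; On BeginPlay the server applies the instigator's magic strength modifier and sets the lifespan, while a locally controlled instigator can get a HUD buff icon.
; Stack functions add, remove and count active spells by SpellID through a magic system interface, lazily cached from the instigator's tagged component.
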(event EventBeginPlay
  (bind _returnvalue (Game|GetInstigator))
  (bind _controller (CallFunction|GetControllerfromActor _returnvalue))
  (Utilities|FlowControl|Sequence
    (:then_0
      (if (Networking|IsServer)
        ;[1 0 0] Will cause error/warning in devkit as magic system component won't be found, this won't happen in game as magic component will be found
        (bind _magicstrengthmodifier (Default|GetPlayerMagicStrengthModifier (CallFunction|GetMagicInterface)))
        (if (> _magicstrengthmodifier 0.0)
          (Variables|Default|SetSpellModifier _magicstrengthmodifier))
        (Actor|SetLifeSpan (Variables|Default|GetLifespan%20))))
    (:then_1
      (Utilities|IsValid _controller
        (:Is%20Valid
          (if (and (Variables|BuffList|GetHasBuffIcon) (Pawn|IsLocalPlayerController _controller))
            (bind _asplayer_controller (Utilities|Casting|CastToPlayerController _controller))
            (bind _ashudinterface (Utilities|Casting|CastToHUDInterface (HUD|GetHUD _asplayer_controller)))
            (Default|AddOtherBuffWidget :self _ashudinterface :Name (Variables|BuffList|GetSpellBuffName) :Icon (Variables|BuffList|GetSpellBuffIcon) :Duration (Variables|BuffList|GetSpellBuffDuration))))))))

(fn ConstructionScript)

(fn GetMagicInterface
  (Utilities|IsInterfaceValid? (Variables|Default|GetMagicSystemInterface)
    (:IsValid
      (return (Variables|Default|GetMagicSystemInterface)))
    (:IsNotValid
      (bind _asi_magic_system (Utilities|Casting|CastToI_MagicSystem (Utilities|Array|Get(acopy) (Actor|GetComponentsbyTag (Game|GetInstigator) "/Script/Engine.ActorComponent" "MagicSystem")))
        (:then
          (bind _output_get (Variables|Default|SetMagicSystemInterface _asi_magic_system))
          (return _output_get))
        (:CastFailed
          (return 0))))))

(fn AddStack
  (Default|AddActiveSpell (CallFunction|GetMagicInterface) (Variables|Default|GetSpellID)))

(fn RemovefromStack
  (Default|RemoveActiveSpell (CallFunction|GetMagicInterface) (Variables|Default|GetSpellID)))

(fn GetStackCount
  (bind _spellstackcount (Default|IsSpellActive (CallFunction|GetMagicInterface) (Variables|Default|GetSpellID)))
  (return _spellstackcount))