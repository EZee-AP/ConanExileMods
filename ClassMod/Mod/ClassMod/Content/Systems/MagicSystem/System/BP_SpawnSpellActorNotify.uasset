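; Animation notify, labeled "Cast Spell", that triggers spawning of its Spell at a chosen point in an animation.
; On the server only, it takes the first component tagged "MagicSystem" on the mesh's owner.
; It calls SpawnSpellFromAnimNotify on that component through the I_MagicSystem interface, leaving the actual spawning to the magic system.
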(fn ReceivedNotify
  (params (MeshComp :type Skeletal%20Mesh%20Component%20Object%20Reference) (Animation :type Anim%20Sequence%20Base%20Object%20Reference))
  (if (Networking|IsServer)
    (bind _asi_magic_system (Utilities|Casting|CastToI_MagicSystem (Utilities|Array|Get(acopy) (Actor|GetComponentsbyTag (Components|GetOwner MeshComp) "/Script/Engine.ActorComponent" "MagicSystem")))
      (:then
        (Default|SpawnSpellfromAnimNotify _asi_magic_system (Variables|Default|GetSpell))
        (return true))
      (:CastFailed
        (return true)))
    (else
      (return true))))

(fn GetNotifyName
  (return "Cast Spell"))