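; Lightning strike AOE spell actor that repeatedly damages Conan characters within a fixed box around it.
; The server runs a half-second timer loop, box-tracing pawns and applying health damage credited to the instigator until StrikeCount runs out, then destroys the actor.
; Clients only time the lightning particle's shutoff from StrikeCount.
; A helper caches the instigator's tagged MagicSystem interface, though no graph here calls it.
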(event Custom|Strike
  (bind _returnvalue (Transformation|GetActorLocation))
  (bind _returnvalue_2 (Game|GetInstigator))
  (bind _returnvalue_3 (+ _returnvalue "0, 0,150.000000"))
  (Math|Integer|DecrementInt (Variables|Default|GetStrikeCount)
    (:%20%20
      (bind _outhits (Class|KismetSystemLibrary|BoxTraceMultiforObjects _returnvalue_3 _returnvalue_3 "200.000000,200.000000,150.000000" (Transformation|GetActorRotation) (Utilities|Array|MakeArray "ObjectTypeQuery3") false 0 "None" true))
      (for _array_element _outhits
        (if (.bSuccess (Utilities|Casting|CastToConanCharacter (.HitActor (Collision|BreakHitResult _array_element))))
          (Game|Damage|ApplyDamage (.AsConan%20Character (Utilities|Casting|CastToConanCharacter (.HitActor (Collision|BreakHitResult _array_element)))) (Variables|Default|GetDamage) (CallFunction|GetControllerfromActor _returnvalue_2) _returnvalue_2 "/Game/Systems/Progression/DmgTypeHealth_BP.DmgTypeHealth_BP_C")))
      (if (> (Variables|Default|GetStrikeCount) 0)
        (Utilities|Time|SetTimerbyFunctionName 0 "DoStrike" 0.5)
        (else
          (Components|Activation|Deactivate (Variables|Default|GetP_Lightning))
          (Utilities|FlowControl|Delay 1.0)
          (Actor|DestroyActor))))))

(event EventBeginPlay
  (if (Networking|IsServer)
    (Utilities|Time|SetTimerbyFunctionName 0 "DoStrike" 0.5)
    (else
      (Utilities|FlowControl|Delay (* (Variables|Default|GetStrikeCount) 0.5))
      (Components|Activation|Deactivate (Variables|Default|GetP_Lightning)))))

(fn ConstructionScript)

(fn DoStrike
  (CallFunction|Strike))

(fn GetMagicInterface
  (Utilities|IsInterfaceValid? (Variables|Default|GetMagicSystemInterface)
    (:IsValid
      (return (Variables|Default|GetMagicSystemInterface)))
    (:IsNotValid
      (bind _asi_magic_system (Utilities|Casting|CastToI_MagicSystem (Utilities|Array|Get(acopy) (Actor|GetComponentsbyTag (Game|GetInstigator) "/Script/Engine.ActorComponent" "MagicSystem")))
        (:then
          (bind _output_get (Variables|Default|SetMagicSystemInterface _asi_magic_system))
          (return _output_get))
        (:CastFailed
          (return 0))))))