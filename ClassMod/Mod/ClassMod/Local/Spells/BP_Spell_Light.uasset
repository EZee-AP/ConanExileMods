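; Light spell buff actor that surrounds the casting player with a tinted force-field mesh and point light, attached at the pelvis socket.
; A timeline scales the mesh and light intensity up on spawn, then reverses when the buff duration expires.
; The server manages stack add and removal and destroys the actor after a short delay.
; Dedicated servers skip all visuals and use only a timer.
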(event Custom|CustomEvent_0
  (Variables|Default|SetDestroy true)
  (bind _newtrack_0 (Timeline|Timeline_0 ReverseFromEnd)
    (:Update
      (Transformation|SetWorldScale3D (Variables|Default|GetSM_ForceField) (* "1.000000,1.000000,1.000000" _newtrack_0))
      (Rendering|Components|Light|SetIntensity (Variables|Default|GetPointLight) (* (Variables|Default|GetLightIntensity) _newtrack_0)))
    (:Finished
      (if (Variables|Default|GetDestroy)
        (if (Networking|IsServer)
          (CallFunction|RemovefromStack)
          (Utilities|FlowControl|Delay 1.0)
          (Actor|DestroyActor))))))

(event Custom|CustomEvent_1
  (CallFunction|RemovefromStack)
  (Actor|DestroyActor))

(event EventBeginPlay
  (bind _lightcolor (Variables|Default|GetLightColor))
  (|CallParentFunction)
  (if (Networking|IsServer)
    (CallFunction|AddStack)
    (if (Networking|IsDedicatedServer)
      (Utilities|Time|SetTimerbyEvent (delegate Custom|CustomEvent_1) (+ (Variables|Default|GetSpellBuffDuration) 1.0))
      (else
        (bind _returnvalue (Rendering|Material|CreateDynamicMaterialInstance (Variables|Default|GetSM_ForceField) 0 "/Game/Mods/ClassMod/Art/M_SpellLight.M_SpellLight" :!class /Script/Engine.PrimitiveComponent :!label _label))
        (Rendering|Material|SetVectorParameterValue _returnvalue "Color" _lightcolor :!class /Script/Engine.MaterialInstanceDynamic)
        (Rendering|Components|Light|SetLightColor (Variables|Default|GetPointLight) _lightcolor true)
        (Transformation|AttachComponentToComponent (Variables|/Script/Engine.Character|GetMesh (.AsBase%20Player%20Char (Utilities|Casting|CastToBasePlayerChar (Game|GetInstigator)))) "b_pelvis" "SnapToTarget" "SnapToTarget" "SnapToTarget" true)
        (Utilities|Time|SetTimerbyEvent (delegate Custom|CustomEvent_0) (Variables|Default|GetSpellBuffDuration))
        (bind _newtrack_0 (Timeline|Timeline_0 PlayFromStart)
          (:Update
            (Transformation|SetWorldScale3D (Variables|Default|GetSM_ForceField) (* "1.000000,1.000000,1.000000" _newtrack_0))
            (Rendering|Components|Light|SetIntensity (Variables|Default|GetPointLight) (* (Variables|Default|GetLightIntensity) _newtrack_0)))
          (:Finished
            (if (Variables|Default|GetDestroy)
              (if (Networking|IsServer)
                (CallFunction|RemovefromStack)
                (Utilities|FlowControl|Delay 1.0)
                (Actor|DestroyActor)))))))
    (else
      (goto _label))))

(fn ConstructionScript
  (|CallParentFunction))