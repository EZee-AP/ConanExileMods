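; BP_Spell_Lightning is a spell actor that calls down a lightning strike where its caster aims.
; On BeginPlay the server runs a ranged sphere aim query, targeting a hit ConanCharacter's feet or otherwise the hit location.
; It spawns BP_LightningStrike there with the caster's aim yaw and modifier-scaled damage, then destroys itself after a short delay.
; A failed query shows the caster a "MISS" notification and destroys the spell immediately.
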(event EventBeginPlay
  (bind _returnvalue (Game|GetInstigator))
  (bind _returnvalue_2 (Game|GetInstigator))
  (bind (_location _hitactor _success) (CallFunction|GetLookatAimHitLocationSphere _returnvalue 3e+03 5e+01))
  (bind (_asconan_character _bsuccess) (Utilities|Casting|CastToConanCharacter _hitactor))
  (|CallParentFunction)
  (if (Networking|IsServer)
    (if _success
      (if (and (Utilities|IsValid _hitactor) _bsuccess)
        (Variables|Default|Setloc (CallFunction|GetActorFeetLocation _asconan_character))
        (else
          (Variables|Default|Setloc _location)))
      (Game|SpawnActorfromClass "/Game/Mods/ClassMod/Spells/AOE/BP_LightningStrike.BP_LightningStrike_C" (Math|Transform|MakeTransform (Variables|Default|Getloc) (Math|Rotator|MakeRotator 0.0 0.0 (.yaw (Pawn|GetBaseAimRotation _returnvalue))) "1,1,1") "AlwaysSpawn" _returnvalue_2 (* (Variables|Default|GetDamage) (Variables|Default|GetSpellModifier)) _returnvalue_2)
      (Utilities|FlowControl|Delay 0.5)
      (Actor|DestroyActor)
      (else
        ;[1 1 1] miss
        (Class|ConanCharacter|ClientHUDShowNotification (.AsConan%20Character (Utilities|Casting|CastToConanCharacter _returnvalue)) (Utilities|Text|MakeLiteralText "MISS") true)
        (Actor|DestroyActor)))))

(fn ConstructionScript
  (|CallParentFunction))