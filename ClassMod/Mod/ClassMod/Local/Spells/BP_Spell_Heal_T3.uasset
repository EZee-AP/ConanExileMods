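; Tier 3 heal spell projectile that delivers a Tier 2 heal at a distance.
; On BeginPlay it moves just in front of the instigator along their aim, then a timeline drives it forward without sweeping.
; The first sphere overlap stops the particles, and the server spawns BP_Spell_Heal_T2 there with the same owner and instigator.
; The server sets a short lifespan on overlap or when the timeline finishes.
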(event OnComponentBeginOverlap(Sphere)
  (params (OverlappedComponent :type Primitive%20Component%20Object%20Reference) (OtherActor :type Actor%20Object%20Reference) (OtherComp :type Primitive%20Component%20Object%20Reference) (OtherBodyIndex :type Integer) (bFromSweep :type Boolean) (SweepResult :type Hit%20Result%20Structure%20%28by%20ref%29))
  (Utilities|FlowControl|DoOnce false
    (:Completed
      (Components|Activation|Deactivate (Variables|Default|GetParticleSystem))
      (if (Networking|IsServer)
        (Game|SpawnActorfromClass "/Game/Mods/ClassMod/Spells/BP_Spell_Heal_T2.BP_Spell_Heal_T2_C" (Math|Transform|MakeTransform (Transformation|GetActorLocation) "0, 0, 0" "1,1,1") "AlwaysSpawn" (Components|GetOwner) (Game|GetInstigator))
        (Actor|SetLifeSpan 3.0)))))

(event EventBeginPlay
  (|CallParentFunction)
  (Transformation|SetActorTransform (CallFunction|GetAdjustedTransform) false true)
  (Collision|SetCollisionEnabled (Variables|Default|GetSphere) "QueryOnly")
  (Variables|Default|SetStartLocation (Transformation|GetActorLocation))
  (bind _newtrack_1 (Timeline|Timeline_0 PlayFromStart)
    (:Update
      (Transformation|SetWorldLocation (Variables|Default|GetDefaultSceneRoot) (+ (Variables|Default|GetStartLocation) (* (Math|Vector|GetForwardVector (Transformation|GetActorRotation)) (* _newtrack_1 1.5e+04))) false false))
    (:Finished
      (Components|Activation|Deactivate (Variables|Default|GetParticleSystem))
      (if (Networking|IsServer)
        (Actor|SetLifeSpan 3.0)))))

(fn ConstructionScript
  (|CallParentFunction))

(fn GetAdjustedTransform
  (bind _returnvalue (Game|GetInstigator))
  (bind _returnvalue_2 (Pawn|GetBaseAimRotation _returnvalue))
  (bind _returnvalue_3 (Math|Vector|GetForwardVector _returnvalue_2))
  (bind _returnvalue_4 (* _returnvalue_3 1.5e+02))
  (return (Math|Transform|MakeTransform (+ (Math|Vector|MakeVector (.x _returnvalue_4) (.y _returnvalue_4) 5e+01) (Transformation|GetActorLocation _returnvalue)) _returnvalue_2 "1,1,1")))