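; Heal spell actor that restores health over time to the player character that instigated it.
; On the server, BeginPlay attaches it to the caster's pelvis socket, adds a stack and applies the first tick.
; Each tick adds health scaled by the spell modifier and re-arms a short timer until the tick count runs out.
; It then removes its stack and destroys itself after a brief delay.
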(event Custom|HealTick
  (bind _maxticks (Variables|Default|GetMaxTicks))
  (Default|AdjustHealth (.AsBase%20Player%20Char (Utilities|Casting|CastToBasePlayerChar (Game|GetInstigator))) (Math|Float|Truncate (* (Variables|Default|GetHealth) (Variables|Default|GetSpellModifier))))
  (Math|Integer|DecrementInt _maxticks
    (:%20%20
      (if (> _maxticks 0)
        (Utilities|Time|SetTimerbyFunctionName 0 "DoHealTick" 0.5)
        (else
          (CallFunction|RemovefromStack)
          (Utilities|FlowControl|Delay 2.0)
          (Actor|DestroyActor))))))

(event EventBeginPlay
  (|CallParentFunction)
  (if (Networking|IsServer)
    (Transformation|AttachComponentToComponent (Variables|/Script/Engine.Character|GetMesh (.AsBase%20Player%20Char (Utilities|Casting|CastToBasePlayerChar (Game|GetInstigator)))) "b_pelvis" "SnapToTarget" "SnapToTarget" "SnapToTarget" true)
    (CallFunction|AddStack)
    (CallFunction|HealTick)
    (Utilities|Time|SetTimerbyFunctionName 0 "DoHealTick" 0.5)))

(fn ConstructionScript
  (|CallParentFunction))

(fn DoHealTick
  (CallFunction|HealTick))