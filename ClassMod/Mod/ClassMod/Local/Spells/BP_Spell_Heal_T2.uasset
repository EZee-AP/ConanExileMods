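; Tier 2 healing spell actor that creates a timed area heal around its location.
; A looping one-second server timer drives healing, with a capsule trace finding nearby player characters and adjusting their health by an amount scaled by SpellModifier.
; Outside dedicated servers, a timeline grows the decal, then reverses after the duration and deactivates the particles.
; The server sets a short lifespan to remove the actor when the spell ends.
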(event Custom|Heal_Tick
  (bind _returnvalue (Transformation|GetActorLocation))
  (bind _outhits (Class|KismetSystemLibrary|CapsuleTraceMultiforObjects _returnvalue _returnvalue 4.5e+02 0.0 (Utilities|Array|MakeArray "ObjectTypeQuery3") false 0 "ForDuration" true))
  (for _array_element _outhits
    (if (Utilities|DoesObjectImplementInterface (.HitActor (Collision|BreakHitResult _array_element)) "/Game/Systems/Interfaces/BasePlayerCharInterface.BasePlayerCharInterface_C")
      (bind _asbase_player_char (Utilities|Casting|CastToBasePlayerChar (.HitActor (Collision|BreakHitResult _array_element))))
      (Default|AdjustHealth _asbase_player_char (Math|Float|Truncate (* (Variables|Default|GetHealth) (Variables|Default|GetSpellModifier)))))))

(event Custom|ReverseTimeline
  (Variables|Default|SetIsEnding true)
  (bind _newtrack_0 (Timeline|Timeline_0 ReverseFromEnd)
    (:Update
      (Transformation|SetWorldScale3D (Variables|Default|GetDecal) (Math|Vector|MakeVector 1.0 (* 1.0 _newtrack_0) (* 1.0 _newtrack_0))))
    (:Finished
      (if (Variables|Default|GetIsEnding)
        (Components|Activation|Deactivate (Variables|Default|GetParticleSystem))
        (if (Networking|IsServer)
          (Actor|SetLifeSpan 1.0))
        (else
          (Utilities|Time|SetTimerbyEvent (EventDispatchers|CreateEvent :!event Custom|ReverseTimeline) (Variables|Default|GetDuraction)))))))

(event Custom|CustomEvent_0
  (Actor|SetLifeSpan 1.0))

(event EventBeginPlay
  (|CallParentFunction)
  (if (Networking|IsServer)
    (Utilities|Time|SetTimerbyEvent (EventDispatchers|CreateEvent :!event Custom|Heal_Tick) 1.0 true)
    (if (Networking|IsDedicatedServer)
      (Development|PrintString "Hello")
      (Utilities|Time|SetTimerbyEvent (delegate Custom|CustomEvent_0) (Variables|Default|GetDuraction))
      (else
        (bind _newtrack_0 (Timeline|Timeline_0 PlayFromStart)
          (:Update
            (Transformation|SetWorldScale3D (Variables|Default|GetDecal) (Math|Vector|MakeVector 1.0 (* 1.0 _newtrack_0) (* 1.0 _newtrack_0))))
          (:Finished
            (if (Variables|Default|GetIsEnding)
              (Components|Activation|Deactivate (Variables|Default|GetParticleSystem))
              (if (Networking|IsServer)
                (Actor|SetLifeSpan 1.0))
              (else
                (Utilities|Time|SetTimerbyEvent (EventDispatchers|CreateEvent :!event Custom|ReverseTimeline) (Variables|Default|GetDuraction))))))))
    (else
      (Timeline|Timeline_0 PlayFromStart))))

(fn ConstructionScript
  (|CallParentFunction))