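; BP_SpellItem_Dev is a usable item that casts the spell mapped to its TemplateID in DT_SpellData_Main.
; On use, the server looks up that row, optionally plays the caster's animation montage, and spawns the spell actor at the caster's transform as owner and instigator.
; It then zeroes the item's replicated durability and calls Cooldown.
; CanUseItem always returns true, so the item itself imposes no use conditions.
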(event EventOnUseItem
  (params (invokingCharacter :type Conan%20Character%20Object%20Reference))
  (Variables|Default|SetInvokingCharacter (.AsBase%20Player%20Char (Utilities|Casting|CastToBasePlayerChar invokingCharacter)))
  (if (Networking|IsServer)
    (bind _returnvalue (Utilities|GetDataTableRow "/Game/Systems/MagicSystem/System/DT_SpellData_Main.DT_SpellData_Main" (Utilities|String|StringToName (Utilities|String|ToString(Integer) (Variables|Default|GetTemplateID))))
      (:then
        (if (.HasAnimation (Utilities|Struct|BreakST_SpellData _returnvalue))
          (Animation|Montage|MontagePlay (Components|SkeletalMesh|GetAnimInstance (Variables|/Script/Engine.Character|GetMesh (Variables|Default|GetInvokingCharacter))) (|GetAnim (Variables|Default|GetInvokingCharacter) (.AnimationData (Utilities|Struct|BreakST_SpellData _returnvalue))) 1.0 "MontageLength" 0.0))
        (Game|SpawnActorfromClass (.SpellActor (Utilities|Struct|BreakST_SpellData _returnvalue)) (Transformation|GetActorTransform (Variables|Default|GetInvokingCharacter)) "AlwaysSpawn" (Variables|Default|GetInvokingCharacter) (Variables|Default|GetInvokingCharacter))
        (Class|GameItem|SetFloatStat "CurrentDurability" 0.0 true)
        (CallFunction|Cooldown)))))

(fn CanUseItem
  (params (invokingCharacter :type Conan%20Character%20Object%20Reference))
  (return true))