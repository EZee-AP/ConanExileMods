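; BP_LevelProp is a demo interactable level prop: a cube with object info and a radial interaction menu.
; The menu shows the object name and offers red and blue recolors, applied locally through a dynamic material instance; client activation turns it green.
; Its "give wood" entry reaches the server through the MAC_LevelProp_RPC component on the local player character, since menu events fire only on the client.
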(event Custom|Client_MakeRed
  (params (menuEntry :type Radial%20Menu%20Entry%20Object%20Reference))
  ;[1 1 1] *UI* client only
  (CallFunction|SetColor)
  (Development|PrintString "Interactable Menu Red"))

(event Custom|SetColor
  (params (ColorIndex :type Integer))
  (bind _returnvalue (Rendering|Material|CreateDynamicMaterialInstance (Variables|Default|GetCube) 0 0 :!class /Script/Engine.PrimitiveComponent))
  (Rendering|Material|SetVectorParameterValue _returnvalue "Color" (Utilities|Select :Index ColorIndex :Option%200 (Variables|Color|GetColorRed) :Option%201 (Variables|Color|GetColorBlue) :Option%202 (Variables|Color|GetColorGreen)) :!class /Script/Engine.MaterialInstanceDynamic))

(event Custom|Client_MakeBlue
  (params (menuEntry :type Radial%20Menu%20Entry%20Object%20Reference))
  ;[1 1 1] *UI* client only
  (CallFunction|SetColor 1)
  (Development|PrintString "Interactable Menu Blue"))

(event Custom|RPC
  (params (menuEntry :type Radial%20Menu%20Entry%20Object%20Reference))
  ;[1 1 1] *UI* client only
  ;;[0 1 0] RPC
  (Default|ServerGiveMeWood (Actor|GetComponentbyClass (Game|GetPlayerCharacter 0) "/Game/Mods/LevelProp/System/MAC_LevelProp_RPC.MAC_LevelProp_RPC_C")))

(event EventClientInteractableActivate
  (params (Component :type Primitive%20Component%20Object%20Reference) (Instigator :type Player%20Controller%20Object%20Reference) (HitIndex :type Integer))
  ;[1 1 1] We only want to set box color on client in demo
  (CallFunction|SetColor 2)
  (Development|PrintString "Client Interactable Activate Green)"))

(event EventInteractableActivate
  (params (Component :type Primitive%20Component%20Object%20Reference) (Instigator :type Player%20Controller%20Object%20Reference) (HitIndex :type Integer) (TriggeredFromRadialWheel :type Boolean))
  (Development|PrintString "Interactable Activate"))

(event EventInteractableMenu
  (params (RadialMenu :type Radial%20Menu%20Object%20Reference) (HitIndex :type Integer))
  ;[1 1 1] *UI* client only
  ;;[1 0 0] Sets RadialMenu name, probably better way to do this
  (CallFunction|SetRadialMenuName)
  (bind _returnvalue (Class|RadialMenu|AddItem RadialMenu "Make Cube Red" "" "/Game/UI/Textures/GUIs/MainRadialMenu/T_MainRadialMenuIconInteract.T_MainRadialMenuIconInteract" "None" -1))
  (EventDispatchers|BindEventtoSignalClicked _returnvalue (delegate Custom|Client_MakeRed))
  (bind _returnvalue_2 (Class|RadialMenu|AddItem RadialMenu "Make Cube Blue" "" "/Game/UI/Textures/GUIs/MainRadialMenu/T_MainRadialMenuIconInteract.T_MainRadialMenuIconInteract" "None" -1))
  (EventDispatchers|BindEventtoSignalClicked _returnvalue_2 (delegate Custom|Client_MakeBlue))
  ;;[0 1 0] RPC
  (bind _returnvalue_3 (Class|RadialMenu|AddItem RadialMenu "Server Give Me Wood" "" "/Game/UI/Textures/GUIs/MainRadialMenu/T_MainRadialMenuIconPickup.T_MainRadialMenuIconPickup" "None" -1))
  (EventDispatchers|BindEventtoSignalClicked _returnvalue_3 (delegate Custom|RPC)))

(fn ConstructionScript)

(fn SetRadialMenuName
  ;[1 1 1] Probably better way to do this
  (bind _returnvalue (Class|GUIModuleController|ActivateModule (Class|GUIModuleController|GetGUIModuleController) "MainRadialMenu" true false))
  (bind _asw_main_radial_menu (Utilities|Casting|CastToW_MainRadialMenu _returnvalue)
    (:then
      (Class|MainRadialMenu|SetObjectLabelText _asw_main_radial_menu (Variables|Default|GetObjectName)))
    (:CastFailed
      _))
  (return))

(fn GetObjectInfo
  (return (Variables|Default|GetObjectName) (Variables|Default|GetHasObjerctInfo) (Variables|Default|GetObjectInfo)))

(fn InteractableDefaultAction
  (return "NONE" 0))

(fn InteractableGetRepairUIModuleName
  (return "None"))

(fn InteractableGetSimpleDisplayText
  (return ""))

(fn InteractableGetUIModuleName
  (return "LevelPropInfo"))

(fn InteractableMenuDisabled
  (return (Variables|Default|GetDisableInteractionMenu)))

(fn IsMenuDisabled
  (return (Variables|Default|GetDisableInteractionMenu)))