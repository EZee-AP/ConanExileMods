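; BP_Tool is a map utility that snaps every PlayerStart to the landscape height.
; Its SetPlayerStartLocationZ event runs a vertical Visibility multi-trace through each start's XY across a very tall range.
; The first hit on an exact LandscapeStreamingProxy class sets the new location, lifted slightly above the surface, so other blocking or overlapping actors are ignored.
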(event Custom|SetPlayerStartLocationZ
  (bind _outactors (Actor|GetAllActorsOfClass "/Script/Engine.PlayerStart"))
  (for _array_element _outactors
    (bind _outhits (Collision|MultiLineTraceByChannel (Math|Vector|MakeVector (.x (Transformation|GetActorLocation _array_element)) (.y (Transformation|GetActorLocation _array_element)) 8e+04) (Math|Vector|MakeVector (.x (Transformation|GetActorLocation _array_element)) (.y (Transformation|GetActorLocation _array_element)) -8e+04) "TraceTypeQuery1" false 0 "None"))
    (bind _array_element_2 (Utilities|Array|ForEachLoopwithBreak _outhits :!label _label)
      (:LoopBody
        (if (== (Utilities|GetClass (.HitActor (Collision|BreakHitResult _array_element_2))) "/Script/Landscape.LandscapeStreamingProxy")
          (Transformation|SetActorLocation _array_element (+ (.Location (Collision|BreakHitResult _array_element_2)) "0, 0,150.000000") false false)
          (goto _label Break))))))

(fn ConstructionScript)