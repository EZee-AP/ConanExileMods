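; BP_GameItem_Scroll is a usable inventory item that teaches the player a crafting recipe.
; Use calls ServerUseItem, which on authority maps the item's TemplateID to a recipe through two data table lookups.
; An unknown recipe, or one already in the recipe inventory, only shows a HUD message.
; Otherwise it consumes one from the stack, sends loot and HUD notifications, and has RecipeManager learn the recipe.
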(event Custom|ServerUseItem
  (params (OtherActor :type Actor%20Object%20Reference))
  (bind _returnvalue (Class|GameItem|GetIntStat "StackSize"))
  (bind _returnvalue_2 (Class|GameItem|GetOwnerInventory))
  ;[1 1 1] ?????
  (if (Ability|HasAuthority OtherActor)
    (bind _asbase_player_char (Utilities|Casting|CastToBasePlayerChar OtherActor)
      (:then
        (bind _returnvalue_3 (Utilities|GetDataTableRow "/Game/Mods/Scrolls/TemplateIDToRecipeID.TemplateIDToRecipeID" (Utilities|String|StringToName (Utilities|String|ToString(Integer) (Variables|Default|GetTemplateID))))
          (:then
            (bind _returnvalue_4 (Utilities|GetDataTableRow "/Game/Items/Recipes/RecipesTable.RecipesTable" (Utilities|String|StringToName (Utilities|String|ToString(Integer) (Utilities|Struct|BreakST_TemplateIDToRecipeID _returnvalue_3))))
              (:then
                (bind _returnvalue_5 (Class|ConanCharacter|GetRecipeInventory _asbase_player_char))
                (if (Class|ItemInventory|HasItembyTemplateID _returnvalue_5 (Utilities|Struct|BreakST_TemplateIDToRecipeID _returnvalue_3) 1)
                  ;[1 1 1] we already know this recipe
                  (Class|ConanCharacter|ClientHUDShowFIFO _asbase_player_char (Utilities|Text|MakeLiteralText "You already know this recipe"))
                  (else
                    (Utilities|FlowControl|Sequence
                      (:then_0
                        ;[1 1 1] Consume item from item stack. If empty, remove item.
                        (if (<= _returnvalue 1)
                          (Class|ItemInventory|RemoveItem _returnvalue_2 (Class|ItemInventory|GetItemIndex _returnvalue_2 self))
                          (else
                            (Class|GameItem|SetIntStat "StackSize" (- _returnvalue 1) true))))
                      (:then_1
                        ;[1 1 1] LootLog
                        (Class|ConanCharacter|ClientHUDLootNotification _asbase_player_char (Variables|Default|GetTemplateID) -1))
                      (:then_2
                        ;[1 1 1] Notify player to learned recipe
                        (Class|ConanCharacter|ClientHUDShowFIFO _asbase_player_char (Utilities|Text|ToText(String) (Utilities|String|Append "Learned " (Utilities|String|ToString(Text) (.RecipeName (Utilities|Struct|BreakRecipeTableRow _returnvalue_4)))))))
                      (:then_3
                        (Class|RecipeManager|ServerLearnRecipe (Variables|/Game/Characters/BasePlayerChar.BasePlayerChar_C|GetRecipeManager _asbase_player_char) (Utilities|Struct|BreakST_TemplateIDToRecipeID _returnvalue_3)))))))
              (:RowNotFound
                ;[1 1 1] no recipe found
                (Class|ConanCharacter|ClientHUDShowFIFO _asbase_player_char (Utilities|Text|MakeLiteralText "Unknown recipe") :!label _label))))
          (:RowNotFound
            (goto _label))))
      (:CastFailed
        (goto _label)))))

(event EventOnUseItem
  (CallFunction|ServerUseItem (Variables|Default|GetOwnerActor)))

(fn CanUseItem
  (return true))