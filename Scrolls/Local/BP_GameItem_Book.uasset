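; BP_GameItem_Book is a usable book item that teaches the player the recipes mapped to its TemplateID.
; On use, an authority-checked event reads the recipe list from a data table, validates each entry against the recipes table and learns any missing from the recipe inventory through RecipeManager.
; If anything new is learned, it consumes one from the stack and notifies the HUD; otherwise it reports the recipes are already known.
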(event Custom|ServerUseItem
  (params (OtherActor :type Actor%20Object%20Reference))
  (bind _returnvalue (Class|GameItem|GetIntStat "StackSize"))
  (bind _returnvalue_2 (Class|GameItem|GetOwnerInventory))
  (Variables|Default|Setconsume false)
  ;[1 1 1] ?????
  (if (Ability|HasAuthority OtherActor)
    (bind _asbase_player_char (Utilities|Casting|CastToBasePlayerChar OtherActor))
    (bind _returnvalue_3 (Utilities|GetDataTableRow "/Game/Mods/Scrolls/TemplateIDToRecipeIDList.TemplateIDToRecipeIDList" (Utilities|String|StringToName (Utilities|String|ToString(Integer) (Variables|Default|GetTemplateID))))
      (:then
        (for _array_element (.RecipeList (Utilities|Struct|BreakST_RecipeBook _returnvalue_3))
          (Utilities|GetDataTableRow "/Game/Items/Recipes/RecipesTable.RecipesTable" (Utilities|String|StringToName (Utilities|String|ToString(Integer) _array_element))
            (:then
              (bind _returnvalue_4 (Class|ConanCharacter|GetRecipeInventory _asbase_player_char))
              (if (not (Class|ItemInventory|HasItembyTemplateID _returnvalue_4 _array_element 1))
                (Class|RecipeManager|ServerLearnRecipe (Variables|/Game/Characters/BasePlayerChar.BasePlayerChar_C|GetRecipeManager _asbase_player_char) _array_element)
                (Variables|Default|Setconsume true)))))
        (if (Variables|Default|Getconsume)
          (Utilities|FlowControl|Sequence
            (:then_0
              ;[1 1 1] Consume item from item stack. If empty, remove item.
              (if (<= _returnvalue 1)
                (Class|ItemInventory|RemoveItem _returnvalue_2 (Class|ItemInventory|GetItemIndex _returnvalue_2 self))
                (else
                  (Class|GameItem|SetIntStat "StackSize" (- _returnvalue 1) true))))
            (:then_1
              ;[1 1 1] LootLog
              (Class|ConanCharacter|ClientHUDLootNotification _asbase_player_char (Variables|Default|GetTemplateID) -1))
            (:then_2
              ;[1 1 1] Notify player to learned recipe
              (Class|ConanCharacter|ClientHUDShowFIFO _asbase_player_char (Utilities|Text|ToText(String) (Utilities|String|Append "Learned " (.Name (Utilities|Struct|BreakST_RecipeBook _returnvalue_3)))))))
          (else
            ;[1 1 1] We already know all recipes in this book
            (Class|ConanCharacter|ClientHUDShowFIFO _asbase_player_char (Utilities|Text|MakeLiteralText (Utilities|Text|ToText(String) (Utilities|String|Append "You already know  " (.Name (Utilities|Struct|BreakST_RecipeBook _returnvalue_3))))))))))))

(event EventOnUseItem
  (CallFunction|ServerUseItem (Variables|Default|GetOwnerActor)))

(fn CanUseItem
  (return true))