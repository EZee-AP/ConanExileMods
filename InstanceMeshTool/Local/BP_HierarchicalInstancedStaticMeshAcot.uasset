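; Actor Blueprint holding a hierarchical instanced static mesh, with editor Blutility events for relocating the actor independently of its instances.
; Construction Script records HomeLocation while it is still zero.
; UpdateTransforms offsets local instance locations by the movement since home, dirtying render state only on the last, then resets home; SetNewHomeLocation accepts a move that carries instances along.
; BeginPlay randomizes the instancing seed.
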(event Custom|UpdateTransforms
  (bind _hierarchicalinstancedstaticmesh (Variables|Default|GetHierarchicalInstancedStaticMesh))
  (bind _returnvalue (Components|InstancedStaticMesh|GetInstanceCount _hierarchicalinstancedstaticmesh))
  (bind _returnvalue_2 (- _returnvalue 1))
  ;[1 1 1] Blutility: will reset instance transforms if you wish to edit the actor location
  (for _index (range 0 _returnvalue_2)
    (Components|InstancedStaticMesh|UpdateInstanceTransform (Variables|Default|GetHierarchicalInstancedStaticMesh) _index (Math|Transform|MakeTransform (+ (.Location (Math|Transform|BreakTransform (.OutInstanceTransform (Components|InstancedStaticMesh|GetInstanceTransform _hierarchicalinstancedstaticmesh _index false)))) (- (Variables|Default|GetHomeLocation) (Transformation|GetActorLocation self))) (.Rotation (Math|Transform|BreakTransform (.OutInstanceTransform (Components|InstancedStaticMesh|GetInstanceTransform _hierarchicalinstancedstaticmesh _index false)))) (.Scale (Math|Transform|BreakTransform (.OutInstanceTransform (Components|InstancedStaticMesh|GetInstanceTransform _hierarchicalinstancedstaticmesh _index false))))) false (== _index _returnvalue_2) false))
  (Variables|Default|SetHomeLocation (Transformation|GetActorLocation self)))

(event Custom|SetNewHomeLocation
  ;[1 1 1] Blutility: will reset instance transforms if you wish to edit the actor location
  ;;[1 1 1] Blutility: sets new actor home location if you wish to move instances
  (Variables|Default|SetHomeLocation (Transformation|GetActorLocation self)))

(event EventBeginPlay
  (Variables|/Script/Engine.InstancedStaticMeshComponent|SetInstancingRandomSeed (Variables|Default|GetHierarchicalInstancedStaticMesh) (Math|Random|RandomInteger 600613)))

(fn ConstructionScript
  (if (Math|Vector|Equal(Vector) (Variables|Default|GetHomeLocation) "0, 0, 0" 0.0001)
    (Variables|Default|SetHomeLocation (Transformation|GetActorLocation self))))