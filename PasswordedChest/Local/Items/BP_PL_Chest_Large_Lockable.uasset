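; Placeable large lockable chest that puts a password dialog flow in front of normal storage interaction.
; Placement, opening, password changes, admin reset, dismantle and return-to-inventory route through the player's MAC_BasePlayerChar_PC component.
; Activation caches its arguments behind an IsInDialog guard, and InteractableActivatePATCH replays them into BPBACStorage.
; The radial menu gains password entries, and the UI module is swapped to ContainerInfoPATCH.
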(event Custom|Reset_Password
  (params (menuEntry :type Radial%20Menu%20Entry%20Object%20Reference))
  ;[0.3741 1 0.8077] Change Password
  (bind _asbase_player_char (Utilities|Casting|CastToBasePlayerChar (Game|GetPlayerCharacter 0)))
  (Default|ClientResetPassword (Utilities|Array|Get(acopy) (Actor|GetComponentsByClass _asbase_player_char "/Game/Mods/PasswordedChest/Components/MAC_BasePlayerChar_PC.MAC_BasePlayerChar_PC_C")) self))

(event Custom|InteractableActivatePATCH
  ;[0.9397 0.4912 1] Interact With Chest
  (Default|InteractableActivate (Variables|Default|GetBP_BAC_Storage) (Variables|Default|GetMyCom) (Variables|Default|GetMyInst) (Variables|Default|GetMyHit) true))

(event Custom|CustomEvent_0
  (params (menuEntry :type Radial%20Menu%20Entry%20Object%20Reference))
  ;[0.3741 1 0.8077] Change Password
  (bind _asbase_player_char (Utilities|Casting|CastToBasePlayerChar (Game|GetPlayerCharacter 0)))
  (Default|ClientonChangePassword (Utilities|Array|Get(acopy) (Actor|GetComponentsByClass _asbase_player_char "/Game/Mods/PasswordedChest/Components/MAC_BasePlayerChar_PC.MAC_BasePlayerChar_PC_C")) self))

(event EventBeginPlay
  (|CallParentFunction))

(event EventInteractableActivate
  (params (Component :type Primitive%20Component%20Object%20Reference) (Instigator :type Player%20Controller%20Object%20Reference) (HitIndex :type Integer) (TriggeredFromRadialWheel :type Boolean))
  ;[0.9397 0.4912 1] Interact With Chest
  (if (Utilities|Array|ContainsItem (Variables|/Game/Systems/Building/BuildingActorComponents/BP_BAC_Storage.BP_BAC_Storage_C|GetPlayersInteractingWithChest (Variables|Default|GetBP_BAC_Storage)) Instigator)
    (Default|CheckState (Variables|Default|GetBP_BAC_Storage) Instigator)
    (elif (not (Variables|/Game/Systems/Building/BuildingActorComponents/BP_BAC_Storage.BP_BAC_Storage_C|GetOpenState (Variables|Default|GetBP_BAC_Storage)))
      (if (not (Variables|Default|GetIsInDialog))
        (Variables|Default|SetIsInDialog true)
        (Variables|Default|SetMyCom Component)
        (Variables|Default|SetMyInst Instigator)
        (Variables|Default|SetMyHit HitIndex)
        (bind _asbase_player_char (Utilities|Casting|CastToBasePlayerChar (Pawn|GetControlledPawn (Variables|Default|GetMyInst))))
        (Default|ServerOpenChestUI (Utilities|Array|Get(acopy) (Actor|GetComponentsByClass _asbase_player_char "/Game/Mods/PasswordedChest/Components/MAC_BasePlayerChar_PC.MAC_BasePlayerChar_PC_C")) self)))))

(event EventReturntoInventory
  (params (menuEntry :type Radial%20Menu%20Entry%20Object%20Reference))
  ;[0.3018 0.5 0.09372] Return To Inventory
  (bind _asbase_player_char (Utilities|Casting|CastToBasePlayerChar (Game|GetPlayerCharacter 0)))
  (Default|ClientReturntoInventoryDialog (Utilities|Array|Get(acopy) (Actor|GetComponentsByClass _asbase_player_char "/Game/Mods/PasswordedChest/Components/MAC_BasePlayerChar_PC.MAC_BasePlayerChar_PC_C")) self))

(event EventOnPlaced
  (params (PlacedBy :type Conan%20Character%20Object%20Reference))
  (bind _self self)
  ;[0.3369 0.4886 1] Open Password dialog on first place
  (|CallParentFunction PlacedBy)
  (Variables|Default|SetPassword "0000")
  (Variables|Default|SetIsInDialog true)
  (bind _asbase_player_char (Utilities|Casting|CastToBasePlayerChar PlacedBy))
  (Development|PrintString (Utilities|String|Append "On Placed: " (Utilities|GetDisplayName _self)) true true "(R=0.000000,G=0.660000,B=1.000000,A=1.000000)" 5.0)
  (Default|ServerChestonPlace (Utilities|Array|Get(acopy) (Actor|GetComponentsByClass _asbase_player_char "/Game/Mods/PasswordedChest/Components/MAC_BasePlayerChar_PC.MAC_BasePlayerChar_PC_C")) _self))

(event EventInteractMenuDismantle
  (params (menuEntry :type Radial%20Menu%20Entry%20Object%20Reference))
  ;[1 0.085 0.085] dismantle
  (bind _asbase_player_char (Utilities|Casting|CastToBasePlayerChar (Game|GetPlayerCharacter 0)))
  (Default|ClientDismantleDialog (Utilities|Array|Get(acopy) (Actor|GetComponentsByClass _asbase_player_char "/Game/Mods/PasswordedChest/Components/MAC_BasePlayerChar_PC.MAC_BasePlayerChar_PC_C")) self))

(event EventInteractableMenu
  (params (RadialMenu :type Radial%20Menu%20Object%20Reference) (HitIndex :type Integer))
  ;[0.3741 1 0.8077] Change Password
  (|CallParentFunction RadialMenu HitIndex)
  (bind _returnvalue (Class|RadialMenu|AddItem RadialMenu "Change Password" "" "/Game/UI/Textures/GUIs/MainRadialMenu/MainRadialMenuIconLocked.MainRadialMenuIconLocked" "None" -1))
  (EventDispatchers|BindEventtoSignalClicked _returnvalue (delegate Custom|CustomEvent_0))
  (bind _asbase_player_char (Utilities|Casting|CastToBasePlayerChar (Game|GetPlayerCharacter 0)))
  (if (Default|IsAdmin _asbase_player_char)
    (bind _returnvalue_2 (Class|RadialMenu|AddItem RadialMenu "Reset Password To \"0000\"" "" "/Game/UI/Textures/GUIs/MainRadialMenu/MainRadialMenuIconLocked.MainRadialMenuIconLocked" "None" -1))
    (EventDispatchers|BindEventtoSignalClicked _returnvalue_2 (delegate Custom|Reset_Password))))

(fn ConstructionScript
  (|CallParentFunction))

(fn InteractableGetUIModuleName
  (return "ContainerInfoPATCH"))