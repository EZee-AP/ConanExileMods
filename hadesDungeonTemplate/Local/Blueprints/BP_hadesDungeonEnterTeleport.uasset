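; Interactable entrance for the Hades dungeon template that teleports the activating player to a random point inside its TargetBox.
; On server-side activation it reads the first MDC_hadesDungeonTemplate actor in the world to decide whether entry requires an item.
; HasItem searches the character's inventories for that template ID and optionally consumes it.
; Players lacking the item get an "Item Required" HUD notification instead of teleporting.
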(event EventInteractableActivate
  (params (Component :type Primitive%20Component%20Object%20Reference) (Instigator :type Player%20Controller%20Object%20Reference) (HitIndex :type Integer) (TriggeredFromRadialWheel :type Boolean))
  ;[1 1 1] ActivateTeleport
  (if (Networking|IsServer)
    (bind _outactors (Actor|GetAllActorsOfClass "/Game/Mods/hadesDungeonTemplate/MDC_hadesDungeonTemplate.MDC_hadesDungeonTemplate_C"))
    (bind _asconan_player_controller (Utilities|Casting|CastToConanPlayerController Instigator))
    (if (Variables|/Game/Mods/hadesDungeonTemplate/MDC_hadesDungeonTemplate.MDC_hadesDungeonTemplate_C|GetRequiresItem (Utilities|Array|Get(acopy) _outactors))
      (bind _asbase_player_char (Utilities|Casting|CastToBasePlayerChar (Pawn|GetControlledPawn _asconan_player_controller)))
      (if (CallFunction|HasItem (Variables|/Game/Mods/hadesDungeonTemplate/MDC_hadesDungeonTemplate.MDC_hadesDungeonTemplate_C|GetRequiredTemplateID (Utilities|Array|Get(acopy) _outactors)) (Variables|/Game/Mods/hadesDungeonTemplate/MDC_hadesDungeonTemplate.MDC_hadesDungeonTemplate_C|GetConsumesItem (Utilities|Array|Get(acopy) _outactors)) _asbase_player_char)
        (Class|ConanPlayerController|TeleportTriggerboxActivated _asconan_player_controller (Class|FuncomGenericLibrary|GetRandomPointinBox (Variables|Default|GetTargetBox)) (Transformation|GetActorRotation (Pawn|GetControlledPawn _asconan_player_controller)) :!label _label)
        (else
          (Class|ConanCharacter|ClientHUDShowNotification _asbase_player_char (Utilities|Text|MakeLiteralText "Item Required") true)))
      (else
        (goto _label)))))

(fn ConstructionScript)

(fn HasItem
  (params (TemplateID :type Integer) (ConsumeItem :type Boolean) (Character :type Conan%20Character%20Object%20Reference))
  (for _array_element (Actor|GetComponentsByClass Character "/Script/ConanSandbox.ItemInventory")
    (if (Class|ItemInventory|HasItembyTemplateID _array_element TemplateID 1)
      (if ConsumeItem
        (Class|ItemInventory|DeleteItemsbyTemplate _array_element TemplateID 1))
      (return true)))
  (return false))

(fn InteractableDefaultAction
  (return "" 0))

(fn InteractableGetRepairUIModuleName
  (return "None"))

(fn InteractableGetSimpleDisplayText
  (return "Enter Hades Dungeon"))

(fn InteractableGetUIModuleName
  (return "SimpleInfo"))

(fn InteractableMenuDisabled
  (return false))

(fn InteractableShouldCommand
  (return false))