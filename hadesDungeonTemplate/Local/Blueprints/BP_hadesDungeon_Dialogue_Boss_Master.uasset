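; Base dialogue NPC for Hades dungeon bosses that can be activated once and vanishes after its conversation ends.
; On the client it watches the NPCDialogueWindow GUI module and reports closing through the player controller's MAC_BossDialogue component.
; Server_ExitDialogue starts a timed sequence: multicast particle, hidden capsule with collision off, then HandleTriggerOnDeath and actor destruction.
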(event Custom|MULTICAST_PlayParticle
  (bind _capsulecomponent (Variables|Default|GetCapsuleComponent))
  ;[1 1 1] PARTICLE
  (Effects|SpawnEmitteratLocation (Variables|BossConfig|GetBoss_Particle) (Transformation|GetActorLocation))
  (Utilities|FlowControl|Delay (Variables|BossConfig|GetNPCVisabilityDelay))
  (Rendering|SetVisibility _capsulecomponent false true)
  (Collision|SetCollisionEnabled _capsulecomponent "NoCollision"))

(event Custom|Server_ExitDialogue
  (Utilities|Time|SetTimerbyEvent (delegate Custom|TimeBeforeParticle) (Variables|BossConfig|GetParticleDelay)))

(event Custom|CustomEvent
  ;[1 1 1] Time Into Particle NPC Will Be Deleted
  (CallFunction|HandleTriggeronDeath)
  (Actor|DestroyActor))

(event Custom|TimeBeforeParticle
  (bind _npcvisabilitydelay (Variables|BossConfig|GetNPCVisabilityDelay))
  (CallFunction|MULTICASTPlayParticle)
  (Utilities|FlowControl|Delay _npcvisabilitydelay)
  (Collision|SetCollisionEnabled (Variables|Default|GetCapsuleComponent) "NoCollision")
  ;[1 1 1] Time Into Particle NPC Will Be Deleted
  (Utilities|Time|SetTimerbyEvent (delegate Custom|CustomEvent) (+ _npcvisabilitydelay 1.0)))

(event Custom|PATCHUI
  (params (module :type GUI%20Module%20Object%20Reference) (isActive :type Boolean))
  ;[1 1 1] Patch UI
  (if (not isActive)
    (Default|ClientExitDialogue (Actor|GetComponentbyClass (Game|GetPlayerController 0) "/Game/Mods/hadesDungeonTemplate/Blueprints/MAC_BossDialogue.MAC_BossDialogue_C") self)
    (bind _returnvalue (Class|GUIModuleController|GetModule (Class|GUIModuleController|GetGUIModuleController) "NPCDialogueWindow"))
    (EventDispatchers|UnbindallEventsfromSignalActivated _returnvalue)))

(event EventBeginPlay
  (|CallParentFunction))

(event EventTick
  (params (DeltaSeconds :type Float%20%28single-precision%29))
  (|CallParentFunction DeltaSeconds))

(event EventClientInteractableActivate
  (params (Component :type Primitive%20Component%20Object%20Reference) (Instigator :type Player%20Controller%20Object%20Reference) (HitIndex :type Integer))
  ;[1 1 1] Patch UI
  (|CallParentFunction Component Instigator HitIndex)
  (bind _returnvalue (Class|GUIModuleController|GetModule (Class|GUIModuleController|GetGUIModuleController) "NPCDialogueWindow"))
  (EventDispatchers|BindEventtoSignalActivated _returnvalue (delegate Custom|PATCHUI)))

(event EventInteractableActivate
  (params (Component :type Primitive%20Component%20Object%20Reference) (Instigator :type Player%20Controller%20Object%20Reference) (HitIndex :type Integer) (TriggeredFromRadialWheel :type Boolean))
  (if (not (Variables|Default|GetEncounterTriggered))
    (Variables|Default|SetEncounterTriggered true)
    (|CallParentFunction Component Instigator HitIndex false)))

(fn ConstructionScript
  (|CallParentFunction))