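; Actor component for the Hades dungeon boss dialogue, relaying dialogue exit and item requirement/reward options between client and server.
; Exit requests reach the server, which forwards them to the boss dialogue NPC.
; Options are read from and saved to the first MDC_hadesDungeonTemplate actor, whose persistence component is marked dirty after edits.
; On load, the server returns values to the client, which fills the cached widget.
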(event Custom|Client_ExitDialogue
  (params (NPC :type Character%20Object%20Reference))
  (CallFunction|ServerExitDialogue NPC))

(event Custom|Client_SaveOptions
  (params (RequiresItem :type Boolean) (ComsumeItem :type Boolean) (RequiredTemplateID :type Integer) (RewardTemplateID :type Integer))
  ;[1 1 1] save
  (CallFunction|ServerSaveOptions RequiresItem ComsumeItem RequiredTemplateID RewardTemplateID))

(event Custom|Server_SaveOptions
  (params (RequiresItem :type Boolean) (ComsumeItem :type Boolean) (RequiredTemplateID :type Integer) (RewardTemplateID :type Integer))
  ;[1 1 1] save
  (bind _outactors (Actor|GetAllActorsOfClass "/Game/Mods/hadesDungeonTemplate/MDC_hadesDungeonTemplate.MDC_hadesDungeonTemplate_C"))
  (Variables|/Game/Mods/hadesDungeonTemplate/MDC_hadesDungeonTemplate.MDC_hadesDungeonTemplate_C|SetRequiresItem (Utilities|Array|Get(acopy) _outactors) RequiresItem)
  (Variables|/Game/Mods/hadesDungeonTemplate/MDC_hadesDungeonTemplate.MDC_hadesDungeonTemplate_C|SetConsumesItem (Utilities|Array|Get(acopy) _outactors) ComsumeItem)
  (Variables|/Game/Mods/hadesDungeonTemplate/MDC_hadesDungeonTemplate.MDC_hadesDungeonTemplate_C|SetRequiredTemplateID (Utilities|Array|Get(acopy) _outactors) RequiredTemplateID)
  (Variables|/Game/Mods/hadesDungeonTemplate/MDC_hadesDungeonTemplate.MDC_hadesDungeonTemplate_C|SetRewardTemplateID (Utilities|Array|Get(acopy) _outactors) RewardTemplateID)
  (Class|PersistenceComponent|SetDirty (Variables|/Script/DreamworldMods.ModController|GetPersistenceComponent (Utilities|Array|Get(acopy) _outactors)) true 5.0))

(event Custom|Server_LoadOptions
  ;[1 1 1] load
  (bind _outactors (Actor|GetAllActorsOfClass "/Game/Mods/hadesDungeonTemplate/MDC_hadesDungeonTemplate.MDC_hadesDungeonTemplate_C"))
  (CallFunction|ClientSetOptions (Variables|/Game/Mods/hadesDungeonTemplate/MDC_hadesDungeonTemplate.MDC_hadesDungeonTemplate_C|GetRequiresItem (Utilities|Array|Get(acopy) _outactors)) (Variables|/Game/Mods/hadesDungeonTemplate/MDC_hadesDungeonTemplate.MDC_hadesDungeonTemplate_C|GetConsumesItem (Utilities|Array|Get(acopy) _outactors)) (Variables|/Game/Mods/hadesDungeonTemplate/MDC_hadesDungeonTemplate.MDC_hadesDungeonTemplate_C|GetRequiredTemplateID (Utilities|Array|Get(acopy) _outactors)) (Variables|/Game/Mods/hadesDungeonTemplate/MDC_hadesDungeonTemplate.MDC_hadesDungeonTemplate_C|GetRewardTemplateID (Utilities|Array|Get(acopy) _outactors))))

(event Custom|Client_SetOptions
  (params (RequiresItem :type Boolean) (ConsumesItem :type Boolean) (RequiredTemplateID :type Integer) (RewardTemplateID :type Integer))
  (bind _widget (Variables|Default|GetWidget))
  ;[1 1 1] load
  (Utilities|IsValid _widget
    (:Is%20Valid
      (Default|LoadOptions _widget RequiresItem ConsumesItem RequiredTemplateID RewardTemplateID))))

(event Custom|Server_ExitDialogue
  (params (NPC :type Character%20Object%20Reference))
  (bind _asbp_hades_dungeon_dialogue_boss_master (Utilities|Casting|CastToBP_hadesDungeon_Dialogue_Boss_Master NPC))
  (Default|ServerExitDialogue _asbp_hades_dungeon_dialogue_boss_master))

(event Custom|Client_LoadOptions
  (params (Widget :type W%20Hades%20Dungeon%20Example%20Widget%20Object%20Reference))
  ;[1 1 1] load
  (Variables|Default|SetWidget Widget)
  (CallFunction|ServerLoadOptions))