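; Boss encounter controller for the Hades dungeon template, driving phases from player presence and Trigger calls.
; The first player entering the outer zone spawns the first territory's enemies; Trigger then advances to the boss spawn, then to defeat.
; Defeat adds the dungeon template's reward item to every listed player's backpack.
; An empty outer zone destroys all spawned NPCs and resets the encounter.
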(event Custom|SpawnBoss
  (Default|SpawnEnemy (Utilities|Array|Get(acopy) (Variables|Default|GetTriggeredTerritories) 1))
  (Variables|Default|SetPhase 2))

(event EventPlayerEntersOuterZone
  (params (PlayerActor :type Actor%20Object%20Reference))
  ;[0.2516 1 0.3114] Player Counter
  ;;[1 1 1] Player entered or left dungeon area
  (Utilities|Array|AddUnique (Variables|/Game/Systems/EncounterControllers/BP_BaseDungeonController.BP_BaseDungeonController_C|GetPlayerListOuter (Variables|Default|GetDungeonController)) PlayerActor)
  (if (not (Variables|Default|GetPhase1Started))
    (CallFunction|EncounterSetup)))

(event EventEncounterReset
  (for _array_element (Variables|Default|GetTriggeredTerritories)
    (for _array_element_2 (Variables|/Game/Systems/Spawning/NPCTerritorySpawner.NPCTerritorySpawner_C|GetSpawnedNPCs _array_element)
      (Actor|DestroyActor _array_element_2)))
  (Variables|Default|SetPhase1Started false)
  (Variables|Default|SetPhase 0)
  (Development|PrintString "reset"))

(event EventEncounterSetup
  (if (> (Utilities|Array|Length (Variables|Default|GetTriggeredTerritories)) 0)
    (Variables|Default|SetPhase1Started true)
    (Variables|Default|SetPhase 1)
    (Default|SpawnEnemy (Utilities|Array|Get(acopy) (Variables|Default|GetTriggeredTerritories)))
    (Development|PrintString "started")))

(event EventPlayerLeavesOuterZone
  (params (PlayerActor :type Actor%20Object%20Reference))
  ;[0.2516 1 0.3114] Player Counter
  ;;[1 1 1] Player entered or left dungeon area
  (Utilities|Array|RemoveItem (Variables|/Game/Systems/EncounterControllers/BP_BaseDungeonController.BP_BaseDungeonController_C|GetPlayerListOuter (Variables|Default|GetDungeonController)) PlayerActor)
  (if (<= (Utilities|Array|Length (Variables|/Game/Systems/EncounterControllers/BP_BaseDungeonController.BP_BaseDungeonController_C|GetPlayerListOuter (Variables|Default|GetDungeonController))) 0)
    (CallFunction|EncounterReset)))

(event EventTrigger
  (params (Data :type STR%20Trigger%20Message%20Structure))
  (switch int (Variables|Default|GetPhase)
    (:1
      (CallFunction|SpawnBoss))
    (:2
      (Variables|Default|SetPhase 3)
      (CallFunction|BossDefeated))))

(event EventBossDefeated
  (bind _dungeoncontroller (Variables|Default|GetDungeonController))
  (bind _playerlistouter (Variables|/Game/Systems/EncounterControllers/BP_BaseDungeonController.BP_BaseDungeonController_C|GetPlayerListOuter _dungeoncontroller))
  (Development|PrintString "Boss Defeated")
  (if (> (Utilities|Array|Length _playerlistouter) 0)
    (bind _outactors (Actor|GetAllActorsOfClass "/Game/Mods/hadesDungeonTemplate/MDC_hadesDungeonTemplate.MDC_hadesDungeonTemplate_C"))
    (for _array_element _playerlistouter
      (bind _asbase_player_char (Utilities|Casting|CastToBasePlayerChar _array_element))
      (bind _returnvalue (Class|ConanCharacter|GetBackpackInventory _asbase_player_char))
      (Class|ItemInventory|AddItemTemplate _returnvalue (Variables|/Game/Mods/hadesDungeonTemplate/MDC_hadesDungeonTemplate.MDC_hadesDungeonTemplate_C|GetRewardTemplateID (Utilities|Array|Get(acopy) _outactors)) -1 1 true 1.0 -1.0))))

(fn ConstructionScript
  (|CallParentFunction))