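; Conan game item, a teleport stone that sends the player using it back to their own bed.
; Use calls SRV_TeleportToBed, which looks up the player's bedroll by unique ID, falls back to the bed, and verifies ownership.
; On success it consumes one from the stack, logs the loss on the HUD and teleports the player just above it.
; Otherwise it shows "Cannot find bed".
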(event Custom|SRV_TeleportToBed
  (params (OtherActor :type Actor%20Object%20Reference))
  (bind _returnvalue (Class|GameItem|GetIntStat "StackSize"))
  (bind _returnvalue_2 (Class|GameItem|GetOwnerInventory))
  (bind _returnvalue_3 (Game|GetGameMode))
  (bind _asbase_player_char (Utilities|Casting|CastToBasePlayerChar OtherActor))
  (Utilities|IsValid _returnvalue_3
    (:Is%20Valid
      ;[1 1 1] try BedrollID
      (bind _actor (Class|BaseGameModeInterface|GetActorbyUniqueIDInterface(Message) _returnvalue_3 (Variables|/Game/Characters/BasePlayerChar.BasePlayerChar_C|GetBedRollID _asbase_player_char)))
      (Utilities|IsValid _actor
        (:Is%20Valid
          (bind _asbuildable_base (Utilities|Casting|CastToBuildableBase _actor))
          (if (Class|BuildableBase|IsOwner _asbuildable_base _asbase_player_char false)
            (Variables|Default|Setloc (Transformation|GetActorLocation _actor))
            (bind _asconan_player_controller (Utilities|Casting|CastToConanPlayerController (Pawn|GetController _asbase_player_char) :!label _label))
            (Utilities|FlowControl|Sequence
              (:then_0
                ;[1 1 1] Consume item from item stack. If empty, remove item.
                (if (<= _returnvalue 1)
                  (Class|ItemInventory|RemoveItem _returnvalue_2 (Class|ItemInventory|GetItemIndex _returnvalue_2 self))
                  (else
                    (Class|GameItem|SetIntStat "StackSize" (- _returnvalue 1) true))))
              (:then_1
                ;[1 1 1] LootLog
                (Class|ConanCharacter|ClientHUDLootNotification _asbase_player_char (Variables|Default|GetTemplateID) -1))
              (:then_2
                (Class|ConanPlayerController|TeleportPlayerServer _asconan_player_controller (Math|Vector|MakeVector (.X (Math|Vector|BreakVector (Variables|Default|Getloc))) (.Y (Math|Vector|BreakVector (Variables|Default|Getloc))) (+ (.Z (Math|Vector|BreakVector (Variables|Default|Getloc))) 1.1e+02)) false false)))
            (else
              ;[1 1 1] if BedrollID invalid try BedID
              (bind _actor_2 (Class|BaseGameModeInterface|GetActorbyUniqueIDInterface(Message) _returnvalue_3 (Variables|/Game/Characters/BasePlayerChar.BasePlayerChar_C|GetBedID _asbase_player_char) :!label _label_2))
              (Utilities|IsValid _actor_2
                (:Is%20Valid
                  (bind _asbuildable_base_2 (Utilities|Casting|CastToBuildableBase _actor_2))
                  (if (Class|BuildableBase|IsOwner _asbuildable_base_2 _asbase_player_char false)
                    (Variables|Default|Setloc (Transformation|GetActorLocation _actor_2))
                    (goto _label)
                    (else
                      _)))
                (:Is%20Not%20Valid
                  _))
              ;[1 1 1] no bed found
              (Class|ConanCharacter|ClientHUDShowFIFO _asbase_player_char (Utilities|Text|MakeLiteralText "Cannot find bed")))))
        (:Is%20Not%20Valid
          (goto _label_2))))))

(event EventOnUseItem
  (CallFunction|SRVTeleporttoBed (Variables|Default|GetOwnerActor)))

(fn CanUseItem
  (return true))