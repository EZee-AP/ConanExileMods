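; BP_HadesBident is the Hades bident weapon, which gradually repairs its own durability over time.
; On the server, Tick restores durability in small steps and switches itself off once the item reaches its maximum.
; A durability stat change below maximum turns Tick back on after a short delay meant to match the tick interval, so it only runs while repair is needed.
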(event EventBeginPlay
  (|CallParentFunction)
  (if (Networking|IsServer)
    (Actor|Tick|SetActorTickEnabled true)))

(event EventTick
  (params (DeltaSeconds :type Float%20%28single-precision%29))
  (bind _owneritem (Variables|Default|GetOwnerItem))
  (if (Networking|IsServer)
    (if (< (Class|GameItem|GetFloatStat _owneritem "CurrentDurability") (Class|GameItem|GetFloatStat _owneritem "MaxDurability"))
      (Class|GameItem|ModifyDurability (Variables|Default|GetOwnerItem) 1.0)
      (else
        (Actor|Tick|SetActorTickEnabled false)))))

(event EventWeaponBroken
  (|CallParentFunction))

(event EventDurabilityFloatStatChanged
  (params (item :type Game%20Item%20Object%20Reference) (statID :type EItemFloatStatID%20Enum :default "WeaponStaminaHeavyChargedRegenModifier") (statValue :type Float%20%28single-precision%29) (deltaValue :type Float%20%28single-precision%29))
  (|CallParentFunction item statID statValue deltaValue)
  (if (Math|Boolean|ANDBoolean (Utilities|Enum|Equal(Enum) statID "CurrentDurability") (not (Class|Actor|IsActorTickEnabled)) (Networking|IsServer))
    (if (< statValue (Class|GameItem|GetFloatStat (Variables|Default|GetOwnerItem) "MaxDurability"))
      ;[1 1 1] Set to Tick Interval
      (Utilities|FlowControl|Delay 3.0)
      (Actor|Tick|SetActorTickEnabled true))))

(fn ConstructionScript
  (|CallParentFunction))