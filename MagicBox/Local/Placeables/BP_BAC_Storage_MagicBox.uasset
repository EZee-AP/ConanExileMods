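; Interactable storage component for the Magic Box placeable, a chest that refills its contents to full stacks.
; Interaction toggles the CraftingGUI per player, with multicast animation and sound as the first opens and the last closes, which also saves the actor.
; Toggling closed runs MaxStacks, rebuilding the inventory from DefaultInventory plus current items, validated against ItemTable, and overriding stack sizes.
; Server_LoadInventory similarly rebuilds it from defaults and the box's saved ItemList.
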(event Custom|CheckState
  (params (Instigator :type Player%20Controller%20Object%20Reference))
  (bind _playersinteractingwithchest (Variables|Default|GetPlayersInteractingWithChest))
  (if (Utilities|Array|ContainsItem (Variables|Default|GetPlayersInteractingWithChest) Instigator)
    (CallFunction|MaxStacks)
    (Utilities|Array|RemoveItem (Variables|Default|GetPlayersInteractingWithChest) Instigator)
    (CallFunction|CloseGui Instigator)
    (if (== (Utilities|Array|Length (Variables|Default|GetPlayersInteractingWithChest)) 0)
      (CallFunction|CloseChest))
    (else
      (if (== (Utilities|Array|Length (Variables|Default|GetPlayersInteractingWithChest)) 0)
        (Utilities|Array|Add _playersinteractingwithchest Instigator)
        (CallFunction|OpenChest)
        (else
          (Utilities|Array|Add _playersinteractingwithchest Instigator)))
      (CallFunction|OpenGui Instigator))))

(event Custom|OpenChest
  (CallFunction|MulticastOpenChest))

(event Custom|CloseChest
  (CallFunction|MulticastCloseChest)
  (Class|WorldPersistenceComponent|SaveActor (Components|GetOwner)))

(event Custom|Multicast_OpenChest
  (bind _sound_open (Variables|Default|GetSound_Open))
  (bind _animinstance (Variables|Default|GetAnimInstance))
  (Utilities|IsValid _animinstance
    (:Is%20Valid
      (Class|BPHasBinaryStatesInterface|SetOpen(Message) _animinstance))
    (:Is%20Not%20Valid
      _))
  (Variables|Default|SetOpenState true)
  (Utilities|IsValid _sound_open
    (:Is%20Valid
      (Audio|PlaySoundatLocation _sound_open (Transformation|GetActorLocation (Components|GetOwner))))))

(event Custom|Multicast_CloseChest
  (bind _animinstance (Variables|Default|GetAnimInstance))
  (bind _sound_close (Variables|Default|GetSound_Close))
  (Utilities|IsValid _animinstance
    (:Is%20Valid
      (Class|BPHasBinaryStatesInterface|SetClosed(Message) _animinstance))
    (:Is%20Not%20Valid
      _))
  (Variables|Default|SetOpenState false)
  (Utilities|IsValid _sound_close
    (:Is%20Valid
      (Audio|PlaySoundatLocation _sound_close (Transformation|GetActorLocation (Components|GetOwner))))))

(event Custom|CloseGui
  (params (Instigator :type Player%20Controller%20Object%20Reference))
  ;[1 1 1] Handle GUI
  (Class|ConanCharacter|SetInteractingActor (.AsConan%20Character (Utilities|Casting|CastToConanCharacter (Pawn|GetControlledPawn Instigator))) 0 "None"))

(event Custom|OpenGui
  (params (Instigator :type Player%20Controller%20Object%20Reference))
  ;[1 1 1] Handle GUI
  (Class|ConanCharacter|SetInteractingActor (.AsConan%20Character (Utilities|Casting|CastToConanCharacter (Pawn|GetControlledPawn Instigator))) (Components|GetOwner) "CraftingGUI"))

(event Custom|CheckStateAndClose
  (params (Instigator :type Player%20Controller%20Object%20Reference))
  (if (Utilities|Array|ContainsItem (Variables|Default|GetPlayersInteractingWithChest) Instigator)
    (Utilities|Array|RemoveItem (Variables|Default|GetPlayersInteractingWithChest) Instigator)
    (if (== (Utilities|Array|Length (Variables|Default|GetPlayersInteractingWithChest)) 0)
      (CallFunction|CloseChest))))

(event Custom|Server_LoadInventory
  (CallFunction|LoadInventoryfromSave))

(event EventBeginPlay
  (bind _returnvalue (Components|GetOwner))
  ;[1 1 1] Begin play
  (Utilities|FlowControl|Sequence
    (:then_0
      (for _array_element (Actor|GetComponentsByClass (Components|GetOwner) "/Script/Engine.SkeletalMeshComponent")
        (Variables|Default|SetAnimInstance (Components|SkeletalMesh|GetAnimInstance _array_element))))
    (:then_1
      (for _array_element_2 (Actor|GetComponentsByClass _returnvalue "/Script/ConanSandbox.ConanBuildingPersistenceComponent")
        (bind _result (|LoadInventory (Class|PersistenceComponent|GetUniqueID _array_element_2))
          (:OnSuccess
            (Class|LoadInventoryCallProxy|ProcessInventoryData _returnvalue _result)))))))

(event EventInteractableActivate
  (params (Component :type Primitive%20Component%20Object%20Reference) (Instigator :type Player%20Controller%20Object%20Reference) (HitIndex :type Integer))
  (CallFunction|CheckState Instigator))

(event EventInteractableSelectionChanged
  (params (IsSelected :type Boolean) (Instigator :type Player%20Controller%20Object%20Reference) (InstanceIndex :type Integer))
  (if (not IsSelected)
    (CallFunction|CheckStateandCLose Instigator)))

(fn MaxStacks
  (bind _asbp_pl_magic_box (Utilities|Casting|CastToBP_PL_MagicBox (Components|GetOwner)))
  (Variables|MagicBox|SetInventory (Variables|/Game/Systems/Building/Placeables/BP_PlaceableItemContainer.BP_PlaceableItemContainer_C|GetPlaceableInventory _asbp_pl_magic_box))
  ;[1 1 1] add default items to list
  (bind _outrownames (DataTable|GetDataTableRowNames "/Game/Items/ItemTable.ItemTable"))
  (Variables|MagicBox|SetTempItemTableRow _outrownames)
  (bind _outrownames_2 (DataTable|GetDataTableRowNames "/Game/Mods/MagicBox/DataTables/DefaultInventory.DefaultInventory"))
  (bind _output_get (Variables|MagicBox|SetTempDefaults _outrownames_2))
  (for _array_element _output_get
    ;;[0 0 1] validate item
    (if (Utilities|Array|ContainsItem (Variables|MagicBox|GetTempItemTableRow) _array_element)
      (Utilities|Array|Add (Variables|MagicBox|GetTempList) (Utilities|NametoInteger _array_element))))
  ;[1 1 1] add current chest inventory to list
  (for _array_element_2 (Variables|/Script/ConanSandbox.ItemInventory|GetItemList (Variables|MagicBox|GetInventory))
    (Utilities|IsValid _array_element_2
      (:Is%20Valid
        (if (not (Utilities|Array|ContainsItem (Variables|MagicBox|GetTempList) (Variables|/Script/ConanSandbox.GameItem|GetTemplateID _array_element_2)))
          (if (Utilities|Array|ContainsItem (Variables|MagicBox|GetTempItemTableRow) (Utilities|IntegertoName (Variables|/Script/ConanSandbox.GameItem|GetTemplateID _array_element_2)))
            (Utilities|Array|Add (Variables|MagicBox|GetTempList) (Variables|/Script/ConanSandbox.GameItem|GetTemplateID _array_element_2)))))))
  ;[1 1 1] replace chest inventory
  (CallFunction|ClearInventory (Variables|MagicBox|GetInventory))
  (for (_array_element_3 _array_index) (Variables|MagicBox|GetTempList)
    (if (< _array_index (Variables|/Script/ConanSandbox.ItemInventory|GetMaxItemCount (Variables|MagicBox|GetInventory)))
      (bind _returnvalue (Utilities|GetDataTableRow "/Game/Items/ItemTable.ItemTable" (Utilities|IntegertoName _array_element_3))
        (:then
          (Class|ItemInventory|AddItemTemplate (Variables|MagicBox|GetInventory) _array_element_3 (Class|ItemInventory|GetFirstFreeIndex (Variables|MagicBox|GetInventory) false) (.MaxStackSize (Utilities|Struct|BreakItemTableRow _returnvalue)) true 1.0 -1.0)))))
  ;[0 1 0] loop through inventory and set all items stack size, includes altars/weapons etc...
  (for _array_element_4 (Variables|/Script/ConanSandbox.ItemInventory|GetItemList (Variables|MagicBox|GetInventory))
    (Utilities|IsValid _array_element_4
      (:Is%20Valid
        (Class|GameItem|SetIntStat _array_element_4 "StackSize" (Variables|Default|Getstacksize) true))))
  ;[1 1 1] cleanup
  (Class|PersistenceComponent|SetDirty (Variables|MagicBox|GetInventory) true)
  (Class|PersistenceComponent|Save (Variables|MagicBox|GetInventory))
  (Utilities|Array|Clear (Variables|MagicBox|GetTempItemTableRow))
  (Utilities|Array|Clear (Variables|MagicBox|GetTempDefaults))
  (Utilities|Array|Clear (Variables|MagicBox|GetTempList)))

(fn LoadInventoryfromSave
  (bind _asbp_pl_magic_box (Utilities|Casting|CastToBP_PL_MagicBox (Components|GetOwner)))
  (bind _output_get (Variables|MagicBox|SetInventory (Variables|/Game/Systems/Building/Placeables/BP_PlaceableItemContainer.BP_PlaceableItemContainer_C|GetPlaceableInventory _asbp_pl_magic_box)))
  (CallFunction|ClearInventory _output_get)
  (bind _outrownames (DataTable|GetDataTableRowNames "/Game/Items/ItemTable.ItemTable"))
  (Variables|MagicBox|SetTempItemTableRow _outrownames)
  (bind _outrownames_2 (DataTable|GetDataTableRowNames "/Game/Mods/MagicBox/DataTables/DefaultInventory.DefaultInventory"))
  ;[1 1 1] add default items
  (bind _output_get_2 (Variables|MagicBox|SetTempDefaults _outrownames_2))
  (for _array_element _output_get_2
    (if (Utilities|Array|ContainsItem (Variables|MagicBox|GetTempItemTableRow) _array_element)
      (bind _returnvalue (Utilities|GetDataTableRow "/Game/Items/ItemTable.ItemTable" _array_element)
        (:then
          (Class|ItemInventory|AddItemTemplate (Variables|MagicBox|GetInventory) (Utilities|NametoInteger _array_element) (Class|ItemInventory|GetFirstFreeIndex (Variables|MagicBox|GetInventory) false) (.MaxStackSize (Utilities|Struct|BreakItemTableRow _returnvalue)) true 1.0 -1.0)))))
  ;[1 1 1] add saved items
  (for (_array_element_2 _array_index) (Variables|/Game/Mods/MagicBox/Placeables/BP_PL_MagicBox.BP_PL_MagicBox_C|GetItemList _asbp_pl_magic_box)
    (if (< _array_index (Variables|/Script/ConanSandbox.ItemInventory|GetMaxItemCount (Variables|MagicBox|GetInventory)))
      (if (not (Utilities|Array|ContainsItem (Variables|MagicBox|GetTempDefaults) (Utilities|IntegertoName _array_element_2)))
        (if (Utilities|Array|ContainsItem (Variables|MagicBox|GetTempItemTableRow) (Utilities|IntegertoName _array_element_2))
          (bind _returnvalue_2 (Utilities|GetDataTableRow "/Game/Items/ItemTable.ItemTable" (Utilities|IntegertoName _array_element_2))
            (:then
              (Class|ItemInventory|AddItemTemplate (Variables|MagicBox|GetInventory) _array_element_2 (Class|ItemInventory|GetFirstFreeIndex (Variables|MagicBox|GetInventory) false) (.MaxStackSize (Utilities|Struct|BreakItemTableRow _returnvalue_2)) true 1.0 -1.0)))))))
  ;[0 1 0] loop threough inventory and set all items to stack size of 100, includes altars/weapons etc...
  (for _array_element_3 (Variables|/Script/ConanSandbox.ItemInventory|GetItemList (Variables|MagicBox|GetInventory))
    (Utilities|IsValid _array_element_3
      (:Is%20Valid
        (Class|GameItem|SetIntStat _array_element_3 "StackSize" (Variables|Default|Getstacksize) true))))
  ;[1 1 1] cleanup
  (Class|PersistenceComponent|SetDirty (Variables|MagicBox|GetInventory) true)
  (Utilities|Array|Clear (Variables|MagicBox|GetTempItemTableRow))
  (Utilities|Array|Clear (Variables|MagicBox|GetTempDefaults)))

(fn ClearInventory
  (params (Inventory :type Item%20Inventory%20Object%20Reference))
  (for _index (range 0 (- (Class|ItemInventory|GetItemCount Inventory) 1))
    (Utilities|IsValid (Class|ItemInventory|GetItem Inventory _index)
      (:Is%20Valid
        (Class|ItemInventory|RemoveItem Inventory _index)))))