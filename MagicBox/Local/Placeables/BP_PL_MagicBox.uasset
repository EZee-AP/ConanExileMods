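; Magic Box placeable whose inventory can be saved and loaded as a list of item types.
; Saving runs a server event that rebuilds ItemList from the unique template IDs in the placeable inventory, while loading is delegated to BPBACStorageMagicBox.
; The "Save List" and "Load List" radial menu entries are disconnected, so InteractableMenu only calls its parent.
; Dedicated server save/load support is still marked as a TODO.
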(event Custom|SaveInventory
  (params (menuEntry :type Radial%20Menu%20Entry%20Object%20Reference))
  ;[1 1 1] TODO add save/load support for dedicated server.....
  (CallFunction|ServerSaveInventory))

(event Custom|Server_SaveInventory
  (bind _itemlist (Variables|MagicBox|GetItemList))
  ;[1 1 1] TODO add save/load support for dedicated server.....
  (Utilities|Array|Clear (Variables|MagicBox|GetItemList))
  (for _array_element (Variables|/Script/ConanSandbox.ItemInventory|GetItemList (Variables|Default|GetPlaceableInventory))
    (if (not (Utilities|Array|ContainsItem _itemlist (Variables|/Script/ConanSandbox.GameItem|GetTemplateID _array_element)))
      (Utilities|Array|Add _itemlist (Variables|/Script/ConanSandbox.GameItem|GetTemplateID _array_element)))))

(event Custom|LoadInventory
  (params (menuEntry :type Radial%20Menu%20Entry%20Object%20Reference))
  ;[1 1 1] TODO add save/load support for dedicated server.....
  (Default|ServerLoadInventory (Variables|MagicBox|GetBP_BAC_Storage_MagicBox)))

(event EventInteractableMenu
  (params (RadialMenu :type Radial%20Menu%20Object%20Reference) (HitIndex :type Integer))
  ;[1 1 1] TODO add save/load support for dedicated server.....
  (|CallParentFunction RadialMenu HitIndex))

(fn ConstructionScript
  (|CallParentFunction))