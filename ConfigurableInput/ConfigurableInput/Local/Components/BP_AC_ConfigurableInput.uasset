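; Actor component that gives the owning player character a rebindable custom key, here showing a "Hello Key" HUD message when pressed.
; On BeginPlay and whenever the Settings GUI module closes, it reads the first key mapped to the "CustomKey" action, keeping the current key if none is found.
; Tick polls that key on player controller 0, using a pressed flag to fire once per press.
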(event Custom|OnSettingsActivatedEvent
  (params (module :type GUI%20Module%20Object%20Reference) (isActive :type Boolean))
  ;[1 1 1] Set initial value for of our key and register event to update the key when settings menu is closed so we can configure the key during game, if mapping is not found in DefaultInput.ini default key value will be used =)
  (if (not isActive)
    ;;[0 1 0] Name of our Input Mapping in DefaultInput.ini
    (bind _returnvalue (Class|FuncomGenericLibrary|GetFirstKeyforActionMapping (Game|GetPlayerController 0) "CustomKey"))
    (if (Utilities|Enum|NotEqual(Enum) (Class|KismetInputLibrary|KeyGetDisplayName _returnvalue) (Utilities|Text|MakeLiteralText "None"))
      (Variables|Default|SetCustomKey _returnvalue))))

(event EventBeginPlay
  ;[1 1 1] Set initial value for of our key and register event to update the key when settings menu is closed so we can configure the key during game, if mapping is not found in DefaultInput.ini default key value will be used =)
  (bind _returnvalue (Class|GUIModuleController|GetModule (Class|GUIModuleController|GetGUIModuleController) "Settings"))
  (EventDispatchers|AssignSignalActivated _returnvalue (delegate Custom|OnSettingsActivatedEvent))
  ;;[0 1 0] Name of our Input Mapping in DefaultInput.ini
  (bind _returnvalue_2 (Class|FuncomGenericLibrary|GetFirstKeyforActionMapping (Game|GetPlayerController 0) "CustomKey"))
  (if (Utilities|Enum|NotEqual(Enum) (Class|KismetInputLibrary|KeyGetDisplayName _returnvalue_2) (Utilities|Text|MakeLiteralText "None"))
    (Variables|Default|SetCustomKey _returnvalue_2)))

(event EventTick
  (params (DeltaSeconds :type Float%20%28single-precision%29))
  (if (Game|Player|IsInputKeyDown (Game|GetPlayerController 0) (Variables|Default|GetCustomKey))
    (if (not (Variables|Default|GetIsPressed))
      (Variables|Default|SetIsPressed true)
      ;[0 1 0] Our key press
      (bind _asbase_player_char (Utilities|Casting|CastToBasePlayerChar (Components|GetOwner)))
      (Class|ConanCharacter|ClientHUDShowFIFO _asbase_player_char (Utilities|Text|MakeLiteralText "Hello Key")))
    (else
      (Variables|Default|SetIsPressed false))))